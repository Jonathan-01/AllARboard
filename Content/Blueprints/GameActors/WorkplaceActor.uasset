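; WorkplaceActor is a Blueprint actor that displays a workplace timer as a radial progress indicator.
; Every Tick, it converts Timer and MaxTimer into an inverted fraction and passes it to SetPercentage.
; SetPercentage lazily creates and caches a dynamic material instance on RadialTimer, then writes the value to its Percentage scalar parameter.
; The graphs only read the timer values and never update them.
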(event `self.ReceiveTick`
  (params (DeltaSeconds :type "Float (single-precision)"))
  (`self.SetPercentage` (- 1.0 (/ (`self.Timer`) (`self.MaxTimer`)))))

(fn `SetPercentage`
  (params (Percentage :type "Float (double-precision)"))
  (`/Engine/EditorBlueprintResources/StandardMacros.IsValid` (`self.Progress`)
    (:`Is Valid`
      _)
    (:`Is Not Valid`
      (bind _returnvalue (`PrimitiveComponent.CreateDynamicMaterialInstance` (`self.RadialTimer`) 0 null "None"))
      (set `self.Progress` _returnvalue)))
  (`MaterialInstanceDynamic.SetScalarParameterValue` (`self.Progress`) "Percentage" (`local.Percentage`)))

(fn `UserConstructionScript`)